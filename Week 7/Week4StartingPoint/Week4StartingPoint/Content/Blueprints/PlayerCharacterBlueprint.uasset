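; Player character Blueprint that drives a held gun spawned through a Child Actor component.
; On BeginPlay it casts the child actor to GunBlueprint and turns off shadow casting on the gun's mesh.
; Fire input shoots along a blend of a random unit vector and the camera forward vector, weighted by the square root of ShotAccuracy.
; The BlueprintReload event forwards reloading to the gun.
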(event EventBeginPlay
  (bind _asgun_blueprint (Utilities|Casting|CastToGunBlueprint (Variables|/Script/Engine.ChildActorComponent|GetChildActor (Variables|Default|GetGun))))
  (Rendering|SetCastShadow (Variables|/Game/Blueprints/GunBlueprint.GunBlueprint_C|GetGun _asgun_blueprint) false))

(event EventBlueprintReload
  (bind _asgun_blueprint (Utilities|Casting|CastToGunBlueprint (Variables|/Script/Engine.ChildActorComponent|GetChildActor (Variables|Default|GetGun))))
  (Default|Reload _asgun_blueprint))

(event Input|ActionEvents|InputActionFire
  (params (Key :type Key%20Structure :default "None"))
  (:Pressed
    (bind _asgun_blueprint (Utilities|Casting|CastToGunBlueprint (Variables|/Script/Engine.ChildActorComponent|GetChildActor (Variables|Default|GetGun))))
    (Default|Fire _asgun_blueprint (Math|Vector|Lerp(Vector) (Math|Random|RandomUnitVector) (Math|Vector|GetForwardVector (Variables|Default|GetCamera)) (Math|Float|Sqrt (Variables|Default|GetShotAccuracy))))))

(fn ConstructionScript)