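; Gun actor with a magazine, a fire-rate cooldown counted down in Tick, and a Reload that refills rounds.
; Fire hits instantly along a predicted projectile path instead of spawning bullets, blending a random vector toward the aim by the square root of accuracy.
; It damages any HealthComponent on the hit actor, plays sound and the parent player's arms montage, and shows debug traces and messages.
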(event EventBeginPlay
  (Variables|Default|SetRoundsRemainingInMagazine%20 (Variables|Default|GetMagazineSize%20)))

(event EventTick
  (params (DeltaSeconds :type Float%20%28single-precision%29))
  (if (not (Variables|Default|GetbCanFire))
    (bind _output_get (Variables|Default|SetTimeTillNextShot (- (Variables|Default|GetTimeTillNextShot) DeltaSeconds)))
    (Variables|Default|SetbCanFire (and (<= _output_get 0.0) (> (Variables|Default|GetRoundsRemainingInMagazine%20) 0)))))

(fn ConstructionScript)

(fn Fire
  (params (LaunchDirection :type Vector))
  (bind _muzzleposition (Variables|Default|GetMuzzlePosition))
  (bind _returnvalue (Transformation|GetWorldLocation _muzzleposition))
  (if (Variables|Default|GetbCanFire)
    (Math|Integer|DecrementInt (Variables|Default|GetRoundsRemainingInMagazine%20)
      (:%20%20
        (Variables|Default|SetbCanFire false)
        (Variables|Default|SetTimeTillNextShot (Variables|Default|GetFIreRate))
        (bind _outhit (Class|GameplayStatics|BlueprintPredictProjectilePathbyTraceChannel _returnvalue (* (Math|Vector|Lerp(Vector) (Math|Random|RandomUnitVector) (Math|Vector|Normalize LaunchDirection) (Math|Float|Sqrt (Variables|Default|GetWeaponAccuracy%20))) (Variables|Default|GetMuzzleVelocity)) true 1.0 "ECC_WorldDynamic" false (Utilities|Array|MakeArray (Components|GetOwner)) "ForDuration" 4.0))
        (Rendering|Debug|DrawDebugLine (Transformation|GetActorLocation) (.location _outhit) "(R=1.000000,G=0.979167,B=0.979167,A=0.300000)" 1.0 1.0)
        (Audio|PlaySoundatLocation "/Game/Assets/Audio/FirstPersonTemplateWeaponFire02.FirstPersonTemplateWeaponFire02" _returnvalue "0, 0, 0" 0.4 1.0 0.0 0 0 0)
        (bind _asplayer_character_blueprint (Utilities|Casting|CastToPlayerCharacterBlueprint (Actor|GetParentActor))
          (:then
            (Animation|Montage|MontagePlay (Components|SkeletalMesh|GetAnimInstance (Variables|/Game/Blueprints/PlayerCharacterBlueprint.PlayerCharacterBlueprint_C|GetArms _asplayer_character_blueprint)) "/Game/Assets/Animations/FirstPersonFire_Montage.FirstPersonFire_Montage" 1.0 "MontageLength" 0.0 true))
          (:CastFailed
            _))
        (if (Utilities|IsValid (.hitactor _outhit))
          (Utilities|IsValid (Actor|GetComponentbyClass (.hitactor _outhit) "/Script/AdvGamesProgramming.HealthComponent")
            (:Is%20Valid
              (Class|HealthComponent|OnTakeDamage (Actor|GetComponentbyClass (.hitactor _outhit) "/Script/AdvGamesProgramming.HealthComponent") (Variables|Default|GetBulletDamage))
              (Development|PrintString (Utilities|String|ToString(Float) (Variables|/Script/AdvGamesProgramming.HealthComponent|GetCurrentHealth (Actor|GetComponentbyClass (.hitactor _outhit) "/Script/AdvGamesProgramming.HealthComponent")))))
            (:Is%20Not%20Valid
              (Development|PrintString "Nothing with health has been hit" :!label _label)))
          (else
            (goto _label)))))))

(fn Reload
  (Variables|Default|SetRoundsRemainingInMagazine%20 (Variables|Default|GetMagazineSize%20)))