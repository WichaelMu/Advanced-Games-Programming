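; Weapon pickup that hands its stats to the gun of the player or enemy character that picks it up, then destroys itself.
; On BeginPlay the authority calls OnGenerate through ServerOnGenerate, then both it and remote instances set the gun mesh material from Rarity.
; OnPickup finds the character's child-actor gun and copies damage, muzzle velocity, magazine size and accuracy, refilling the magazine.
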(event Custom|ServerOnGenerate
  (bind _gunmesh (Variables|Default|GetGunMesh))
  (if (Networking|IsServer)
    (Class|Pickup|OnGenerate)
    (switch Utilities|FlowControl|Switch|SwitchonEWeaponPickupRarity (Variables|Default|GetRarity)
      (:LEGENDARY
        (Rendering|Material|SetMaterial _gunmesh 0 "/Game/Materials/RarityColours/LEGENDARY.LEGENDARY"))
      (:MASTER
        (Rendering|Material|SetMaterial _gunmesh 0 "/Game/Materials/RarityColours/MASTER.MASTER"))
      (:RARE
        (Rendering|Material|SetMaterial _gunmesh 0 "/Game/Materials/RarityColours/RARE.RARE"))
      (:COMMON
        (Rendering|Material|SetMaterial _gunmesh 0 "/Game/Materials/RarityColours/COMMON.COMMON")))))

(event EventBeginPlay
  (bind _gunmesh (Variables|Default|GetGunMesh))
  (Networking|SwitchHasAuthority
    (:Authority
      (CallFunction|ServeronGenerate))
    (:Remote
      (switch Utilities|FlowControl|Switch|SwitchonEWeaponPickupRarity (Variables|Default|GetRarity)
        (:LEGENDARY
          (Rendering|Material|SetMaterial _gunmesh 0 "/Game/Materials/RarityColours/LEGENDARY.LEGENDARY"))
        (:MASTER
          (Rendering|Material|SetMaterial _gunmesh 0 "/Game/Materials/RarityColours/MASTER.MASTER"))
        (:RARE
          (Rendering|Material|SetMaterial _gunmesh 0 "/Game/Materials/RarityColours/RARE.RARE"))
        (:COMMON
          (Rendering|Material|SetMaterial _gunmesh 0 "/Game/Materials/RarityColours/COMMON.COMMON"))))))

(event EventOnPickup
  (params (ActorThatPickedUp :type Actor%20Object%20Reference))
  (bind _asplayer_character_blueprint (Utilities|Casting|CastToPlayerCharacterBlueprint ActorThatPickedUp)
    (:then
      (bind _asgun_blueprint (Utilities|Casting|CastToGunBlueprint (Variables|/Script/Engine.ChildActorComponent|GetChildActor (Variables|/Game/Blueprints/PlayerCharacterBlueprint.PlayerCharacterBlueprint_C|GetGun _asplayer_character_blueprint))))
      (Variables|Default|SetAttachedGun _asgun_blueprint))
    (:CastFailed
      (bind _asenemy_character_blueprint (Utilities|Casting|CastToEnemyCharacterBlueprint ActorThatPickedUp))
      (bind _asgun_blueprint_2 (Utilities|Casting|CastToGunBlueprint (Variables|/Script/Engine.ChildActorComponent|GetChildActor (Variables|/Game/Blueprints/EnemyCharacterBlueprint.EnemyCharacterBlueprint_C|GetGun _asenemy_character_blueprint))))
      (Variables|Default|SetAttachedGun _asgun_blueprint_2)))
  (Variables|/Game/Blueprints/GunBlueprint.GunBlueprint_C|SetBulletDamage (Variables|Default|GetAttachedGun) (Variables|Default|GetBulletDamage))
  (Variables|/Game/Blueprints/GunBlueprint.GunBlueprint_C|SetMuzzleVelocity (Variables|Default|GetAttachedGun) (Variables|Default|GetMuzzleVelocity))
  (bind _output_get (Variables|/Game/Blueprints/GunBlueprint.GunBlueprint_C|SetMagazineSize%20 (Variables|Default|GetAttachedGun) (Variables|Default|GetMagazineSize)))
  (Variables|/Game/Blueprints/GunBlueprint.GunBlueprint_C|SetRoundsRemainingInMagazine%20 (Variables|Default|GetAttachedGun) _output_get)
  (Variables|/Game/Blueprints/GunBlueprint.GunBlueprint_C|SetWeaponAccuracy%20 (Variables|Default|GetAttachedGun) (Variables|Default|GetWeaponAccuracy))
  (Actor|DestroyActor))

(fn ConstructionScript)